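; BP_Enemy is an enemy character that attacks with a sword montage and ragdolls on death.
; Incoming damage is subtracted from a stat on its BPCStats component.
; Begin and End sword trace events toggle a looping timer that sphere-traces between two points for pawns, applying SwordDamage through a DoOnce that resets after a short delay.
; Die disables movement, enables mesh physics and stops further trace hits.
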(event Custom|Damage%20Trace
  ;[0.15 0.15 0.15 0.5] Sword Traces
  (if (not (Variables|Default|GetisDead?))
    (bind (_outhit _returnvalue) (Collision|SphereTraceForObjects (Transformation|GetWorldLocation (Variables|Default|GetStart%20Sword%20Trace%20Pos)) (Transformation|GetWorldLocation (Variables|Default|GetEnd%20Sword%20Trace%20Pos)) 25.0 (Utilities|Array|MakeArray "ObjectTypeQuery3") false 0 "ForOneFrame"))
    (if _returnvalue
      (Utilities|FlowControl|DoOnce false :!label _label
        (:Completed
          (Game|Damage|ApplyDamage (.HitActor (Collision|BreakHitResult _outhit)) (Variables|Default|GetswordDamage) 0 0)
          (Utilities|FlowControl|Delay 0.3)
          (goto _label Reset))))))

(event EventBeginSwordTrace
  ;[0.15 0.15 0.15 0.5] Sword Traces
  (bind _returnvalue (Utilities|Time|SetTimerbyEvent (delegate Custom|Damage%20Trace) 0.01 true)))

(event EventEndSwordTrace
  ;[0.15 0.15 0.15 0.5] Sword Traces
  (if (Utilities|Time|IsValidTimerHandle (stale EventBeginSwordTrace _returnvalue))
    (Utilities|Time|ClearandInvalidateTimerbyHandle (stale EventBeginSwordTrace _returnvalue))))

(event Game|Damage|EventAnyDamage
  (params (Damage :type Float%20%28single-precision%29) (DamageType :type Damage%20Type%20Object%20Reference) (InstigatedBy :type Controller%20Object%20Reference) (DamageCauser :type Actor%20Object%20Reference))
  (Default|IncreaseValue (Variables|Default|GetBPC_Stats) "NewEnumerator0" (* Damage -1.0)))

(event EventDie
  (Pawn|Components|CharacterMovement|DisableMovement (Variables|Character|GetCharacterMovement))
  (Physics|SetSimulatePhysics (Variables|Character|GetMesh) true)
  (Variables|Default|SetisDead? true))

(fn ConstructionScript)

(fn SwordAttack
  (bind _returnvalue (Animation|PlayAnimMontage "/Game/Characters/BOR_Character/Combat/SwordAttackCombo_Montage.SwordAttackCombo_Montage" 1.0 "None"))
  (return _returnvalue))