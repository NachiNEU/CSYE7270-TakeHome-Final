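; AI controller for an enemy that chases targets it perceives.
; On BeginPlay it uses the BD_AI blackboard and runs the BT_Enemy behavior tree.
; AI Perception updates write the sensed actor and a seeing-target flag to the blackboard, and clear both keys when a stimulus is not successfully sensed.
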(event OnTargetPerceptionUpdated(AIPerception)
  (params (Actor :type Actor%20Object%20Reference) (Stimulus :type AI%20Stimulus%20Structure))
  ;[0.15 0.15 0.15 0.5] Chase Logic
  (if (.bSuccessfullySensed (Utilities|Struct|BreakAIStimulus Stimulus))
    (AI|Components|Blackboard|SetValueasBool (AI|GetBlackboard 0) (Utilities|Name|MakeLiteralName "seeingTarget?") true)
    (AI|Components|Blackboard|SetValueasObject (AI|GetBlackboard 0) (Utilities|Name|MakeLiteralName "targetActor") Actor)
    (else
      (AI|Components|Blackboard|ClearValue (AI|GetBlackboard 0) (Utilities|Name|MakeLiteralName "targetActor"))
      (AI|Components|Blackboard|ClearValue (AI|GetBlackboard 0) (Utilities|Name|MakeLiteralName "seeingTarget?")))))

(event EventBeginPlay
  ;[0.15 0.15 0.15 0.5] Set up Blacboard and Behavior Tree
  (Class|AIController|UseBlackboard "/Game/AI/BD_AI.BD_AI")
  (AI|RunBehaviorTree "/Game/AI/BT_Enemy.BT_Enemy"))

(fn ConstructionScript)